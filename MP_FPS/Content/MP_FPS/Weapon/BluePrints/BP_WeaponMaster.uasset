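; BP_WeaponMaster is a multiplayer FPS weapon base supporting hitscan or projectile fire with separate first-person and third-person meshes.
; Client firing sphere-traces from the camera, then from the muzzle toward that point, and sends the result to the server.
; Hitscan applies server damage; projectile mode spawns a first-person projectile client-side and a third-person one server-side.
; A multicast plays fire sound, owner-filtered muzzle flashes and hitscan impact effects.
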(event `Server_ShootInfo`
  (params (HitTResult :type "HitResult Structure") (Hit :type Boolean))
  (bind (_bblockinghit _binitialoverlap _time _location _impactpoint _normal _impactnormal _physmat _hitactor _hitcomponent _hitbonename _hititem _faceindex _tracestart _traceend) (`GameplayStatics.BreakHitResult` HitTResult))
  (bind _returnvalue (`SceneComponent.GetSocketLocation` (`self.SK_TP_WeaponMesh`) (`self.MuzzleSocketName`)))
  (if (`self.HitScan?`)
    (`GameplayStatics.ApplyDamage` _hitactor (`KismetMathLibrary.Conv_IntToDouble` (`self.Damage`)) (`self.GetInstigatorController`) self)
    (else
      (`|SpawnActorFromClass` "/Game/MP_FPS/Weapon/BluePrints/BP_TP_ProjectileMaster.BP_TP_ProjectileMaster_C" (`KismetMathLibrary.MakeTransform` _returnvalue (`KismetMathLibrary.FindLookAtRotation` _returnvalue (`KismetMathLibrary.SelectVector` _impactpoint _traceend)) (1.0 1.0 1.0)) "AlwaysSpawn" "OverrideRootScale" (`self.GetOwner`) (`self.GetInstigator`))))
  (`self.MulticastWeaponFX` HitTResult Hit))

(event `client_Start_firing`
  (bind _bp_charactermaster (`self.BP_CharacterMaster`))
  (bind _fps_cam (`/Game/MP_FPS/character/BP_Character_Master_Auto3.FPS_Cam` _bp_charactermaster))
  (bind _returnvalue (`SceneComponent.K2_GetComponentLocation` _fps_cam))
  (bind (_outhit _returnvalue_2) (`KismetSystemLibrary.SphereTraceSingle` _returnvalue (+ _returnvalue (* (`KismetMathLibrary.GetForwardVector` (`SceneComponent.K2_GetComponentRotation` _fps_cam)) (`self.SphereTraceRange`))) (`self.SphereTraceRadius`) "TraceTypeQuery1" false (`|MakeArray` _bp_charactermaster :!type "Actor Object Reference")))
  (bind (_bblockinghit _binitialoverlap _time _location _impactpoint _normal _impactnormal _physmat _hitactor _hitcomponent _hitbonename _hititem _faceindex _tracestart _traceend) (`GameplayStatics.BreakHitResult` _outhit))
  (bind (_outhit_2 _returnvalue_3) (`KismetSystemLibrary.SphereTraceSingle` (`SceneComponent.GetSocketLocation` (`self.SK_FP_WeaponMesh`) (`self.MuzzleSocketName`)) (`KismetMathLibrary.SelectVector` _impactpoint _traceend _returnvalue_2) (`self.SphereTraceRadius`) "TraceTypeQuery1"))
  (if (not (`self.HitScan?`))
    (`self.Client_ShootInfo` _outhit_2 _returnvalue_3))
  (`self.Server_ShootInfo` _outhit_2 _returnvalue_3))

(event `Client_ShootInfo`
  (params (`Hit Result` :type "HitResult Structure") (Hit :type Boolean))
  (bind (_bblockinghit _binitialoverlap _time _location _impactpoint _normal _impactnormal _physmat _hitactor _hitcomponent _hitbonename _hititem _faceindex _tracestart _traceend) (`GameplayStatics.BreakHitResult` `Hit Result`))
  (bind _returnvalue (`SceneComponent.GetSocketLocation` (`self.SK_FP_WeaponMesh`) (`self.MuzzleSocketName`)))
  (if (not (`self.HitScan?`))
    (`|SpawnActorFromClass` "/Game/MP_FPS/Weapon/BluePrints/BP_FP_ProjectileMaster.BP_FP_ProjectileMaster_C" (`KismetMathLibrary.MakeTransform` _returnvalue (`KismetMathLibrary.FindLookAtRotation` _returnvalue (`KismetMathLibrary.SelectVector` _impactpoint _traceend Hit))) "AlwaysSpawn" "OverrideRootScale" (`self.GetOwner`) (`self.GetInstigator`))))

(event `Client_Stop_Firing`)

(event `MulticastWeaponFX`
  (params (HitTResult :type "HitResult Structure") (Hit :type Boolean))
  (bind (_bblockinghit _binitialoverlap _time _location _impactpoint _normal _impactnormal) (`GameplayStatics.BreakHitResult` HitTResult))
  (bind _ps_muzzleflash (`self.PS_MuzzleFlash`))
  (bind _muzzlesocketname (`self.MuzzleSocketName`))
  (bind _sk_fp_weaponmesh (`self.SK_FP_WeaponMesh`))
  (`GameplayStatics.SpawnSoundAttached` (`self.FireWeaponSound`) _sk_fp_weaponmesh)
  (`|ExecutionSequence`
    (:`then_0`
      (bind _returnvalue (`GameplayStatics.SpawnEmitterAttached` _ps_muzzleflash _sk_fp_weaponmesh _muzzlesocketname))
      (`PrimitiveComponent.SetOnlyOwnerSee` _returnvalue true)
      (if (`self.HitScan?`)
        (if Hit
          (`GameplayStatics.SpawnSoundAtLocation` (`self.ImpactSound`) _impactpoint)
          (`GameplayStatics.SpawnEmitterAtLocation` (`self.PS_Impact`) _impactpoint (`KismetMathLibrary.MakeRotFromZ` _impactnormal)))))
    (:`then_1`
      (bind _returnvalue_2 (`GameplayStatics.SpawnEmitterAttached` _ps_muzzleflash (`self.SK_TP_WeaponMesh`) _muzzlesocketname))
      (`PrimitiveComponent.SetOwnerNoSee` _returnvalue_2 true))))

(fn `UserConstructionScript`)