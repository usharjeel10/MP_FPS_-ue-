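; Master projectile Blueprint for multiplayer FPS weapons that handles impact effects and its own removal.
; On BeginPlay, the authority makes the collision component ignore the instigator while moving.
; A hit calls a server event, which passes the result to a multicast event and destroys the actor after a short delay.
; The multicast spawns impact sound and particles at the hit point, orienting the particles to the surface normal.
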(event `self.ReceiveBeginPlay`
  (`|ExecutionSequence`
    (:`then_0`
      (`/Engine/EditorBlueprintResources/ActorMacros.Switch Has Authority`
        (:`Authority`
          (`PrimitiveComponent.IgnoreActorWhenMoving` (`self.ProjectileCollision`) (`self.GetInstigator`) true))))))

(event `self.ReceiveHit`
  (params (MyComp :type "PrimitiveComponent Object Reference") (Other :type "Actor Object Reference") (OtherComp :type "PrimitiveComponent Object Reference") (bSelfMoved :type Boolean) (HitLocation :type "Vector Structure") (HitNormal :type "Vector Structure") (NormalImpulse :type "Vector Structure") (Hit :type "HitResult Structure (by ref)"))
  (`self.Server_Onhit` Hit))

(event `Server_Onhit`
  (params (HitResult :type "HitResult Structure"))
  (`self.MulticastFX` HitResult)
  (`KismetSystemLibrary.Delay` 0.1)
  (`self.K2_DestroyActor`))

(event `MulticastFX`
  (params (HitResult :type "HitResult Structure"))
  (bind (_bblockinghit _binitialoverlap _time _location _impactpoint _normal _impactnormal) (`GameplayStatics.BreakHitResult` HitResult))
  (`GameplayStatics.SpawnSoundAtLocation` (`self.ImpactSound`) _impactpoint)
  (`GameplayStatics.SpawnEmitterAtLocation` (`self.PS_Impact`) _impactpoint (`KismetMathLibrary.MakeRotFromZ` _impactnormal)))

(fn `UserConstructionScript`)